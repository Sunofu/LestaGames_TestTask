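; Wind trap actor that pushes the player character inside its collider with randomly changing horizontal gusts.
; A looping timer rerolls the wind vector every two seconds and rotates the Direction component to match it.
; Overlap starts a faster looping timer that repeatedly applies the wind through additive LaunchCharacter calls.
; When the tagged player leaves, that timer pauses itself and zeroes the character's horizontal velocity.
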(event OnComponentBeginOverlap(colider)
  (params (OverlappedComponent :type Primitive%20Component%20Object%20Reference) (OtherActor :type Actor%20Object%20Reference) (OtherComp :type Primitive%20Component%20Object%20Reference) (OtherBodyIndex :type Integer) (bFromSweep :type Boolean) (SweepResult :type Hit%20Result%20Structure%20%28by%20ref%29))
  (bind _asbp_lesta_base_character (Utilities|Casting|CastToBP_Lesta_Base_Character OtherActor))
  (Variables|Default|SetIsPlayerInWindZone true)
  (bind _returnvalue (Utilities|Time|SetTimerbyEvent (delegate Custom|WIndStart) 0.2 true)))

(event OnComponentEndOverlap(colider)
  (params (OverlappedComponent :type Primitive%20Component%20Object%20Reference) (OtherActor :type Actor%20Object%20Reference) (OtherComp :type Primitive%20Component%20Object%20Reference) (OtherBodyIndex :type Integer))
  (if (Actor|ActorHasTag OtherActor "Player")
    (Variables|Default|SetIsPlayerInWindZone false)))

(event Custom|ChangeWindDirection
  (bind _returnvalue (Math|Random|RandomUnitVector))
  (bind _windstrength (Variables|Default|GetWindStrength))
  (bind _returnvalue_2 (* _returnvalue _windstrength))
  (bind _output_get (Variables|Default|SetWindDirection (Math|Vector|MakeVector (.x _returnvalue_2) (.y _returnvalue_2) 0.0)))
  (Transformation|SetWorldRotation (Variables|Default|Getdirection) (Math|Rotator|MakeRotfromX _output_get) false false))

(event Custom|WIndStart
  (if (Variables|Default|GetIsPlayerInWindZone)
    (Character|LaunchCharacter (stale OnComponentBeginOverlap(colider) _asbp_lesta_base_character) (Variables|Default|GetWindDirection) false false)
    (else
      (Utilities|Time|PauseTimerbyHandle (stale OnComponentBeginOverlap(colider) _returnvalue))
      (Character|LaunchCharacter (stale OnComponentBeginOverlap(colider) _asbp_lesta_base_character) "0, 0, 0" true false))))

(event EventBeginPlay
  (bind _returnvalue (Math|Random|RandomUnitVector))
  (bind _returnvalue_2 (Math|Rotator|MakeRotfromX _returnvalue))
  (Transformation|SetWorldRotation (Variables|Default|Getdirection) (Math|Rotator|MakeRotator (.roll _returnvalue_2) (.pitch _returnvalue_2) 0.0) false false)
  (Utilities|Time|SetTimerbyEvent (delegate Custom|ChangeWindDirection) 2.0 true))

(fn ConstructionScript)