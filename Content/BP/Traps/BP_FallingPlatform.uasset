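; BP_FallingPlatform is a one-shot trap platform that falls and disappears after a Player-tagged actor overlaps its Box.
; The first overlap swaps the mesh to M_DamageTrap and starts a Timeline that moves the mesh on Z.
; A Delay chained from that Timeline's Update starts the Falling timeline, which drives the mesh's relative location.
; When Falling finishes, the actor destroys itself after a short pause.
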(event OnComponentBeginOverlap(Box)
  (params (OverlappedComponent :type Primitive%20Component%20Object%20Reference) (OtherActor :type Actor%20Object%20Reference) (OtherComp :type Primitive%20Component%20Object%20Reference) (OtherBodyIndex :type Integer) (bFromSweep :type Boolean) (SweepResult :type Hit%20Result%20Structure%20%28by%20ref%29))
  (if (Actor|ActorHasTag OtherActor "Player")
    (if (not (Variables|Default|GetIsActivated))
      (Variables|Default|SetIsActivated true)
      (Rendering|Material|SetMaterial (Variables|Default|GetStaticMesh) 0 "/Game/Materials/M_DamageTrap.M_DamageTrap")
      (bind _newlocation (Timeline|Timeline PlayFromStart)
        (:Update
          (Transformation|SetRelativeLocation (Variables|Default|GetStaticMesh) (Math|Vector|MakeVector 0.0 0.0 _newlocation) false false)
          (Utilities|FlowControl|Delay 1.5)
          (bind _newlocation_2 (Timeline|Falling PlayFromStart)
            (:Update
              (Transformation|SetRelativeLocation (Variables|Default|GetStaticMesh) _newlocation_2 false false))
            (:Finished
              (Utilities|FlowControl|Delay 0.5)
              (Actor|DestroyActor))))))))

(fn ConstructionScript)