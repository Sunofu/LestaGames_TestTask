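; BP_SwingHammer is a trap hammer that swings and knocks player characters away on contact.
; On BeginPlay a timeline plays forward or in reverse depending on IsClockwiseRotation, driving the Handle's roll scaled by MaxRotate.
; Two overlap spheres launch any BP_Lesta_Base_Character along their paired arrow's forward direction with slight lift.
; Only the Sphere1 launch overrides the character's existing velocity; the Sphere launch adds to it.
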(event OnComponentBeginOverlap(Sphere)
  (params (OverlappedComponent :type Primitive%20Component%20Object%20Reference) (OtherActor :type Actor%20Object%20Reference) (OtherComp :type Primitive%20Component%20Object%20Reference) (OtherBodyIndex :type Integer) (bFromSweep :type Boolean) (SweepResult :type Hit%20Result%20Structure%20%28by%20ref%29))
  (bind _arrow (Variables|Default|GetArrow))
  (bind _returnvalue (Transformation|GetWorldRotation _arrow))
  (bind _returnvalue_2 (Math|Vector|GetForwardVector _returnvalue))
  (bind _returnvalue_3 (* _returnvalue_2 1e+03))
  (bind _asbp_lesta_base_character (Utilities|Casting|CastToBP_Lesta_Base_Character OtherActor))
  (Character|LaunchCharacter _asbp_lesta_base_character (Math|Vector|MakeVector (.x _returnvalue_3) (.y _returnvalue_3) (+ (.z _returnvalue_3) 1e+01)) false false))

(event OnComponentBeginOverlap(Sphere1)
  (params (OverlappedComponent :type Primitive%20Component%20Object%20Reference) (OtherActor :type Actor%20Object%20Reference) (OtherComp :type Primitive%20Component%20Object%20Reference) (OtherBodyIndex :type Integer) (bFromSweep :type Boolean) (SweepResult :type Hit%20Result%20Structure%20%28by%20ref%29))
  (bind _arrow1 (Variables|Default|GetArrow1))
  (bind _returnvalue (Transformation|GetWorldRotation _arrow1))
  (bind _returnvalue_2 (Math|Vector|GetForwardVector _returnvalue))
  (bind _returnvalue_3 (* _returnvalue_2 1e+03))
  (bind _asbp_lesta_base_character (Utilities|Casting|CastToBP_Lesta_Base_Character OtherActor))
  (Character|LaunchCharacter _asbp_lesta_base_character (Math|Vector|MakeVector (.x _returnvalue_3) (.y _returnvalue_3) (+ (.z _returnvalue_3) 1e+01)) true true))

(event EventBeginPlay
  (if (Variables|Default|GetIsClockwiseRotation)
    (bind _newtrack_1 (Timeline|SwingTimeLine PlayFromStart)
      (:Update
        (Variables|Default|SetRotationValue _newtrack_1)
        (Transformation|SetRelativeRotation (Variables|Default|Gethandle) (Math|Rotator|MakeRotator (* (Variables|Default|GetRotationValue) (Variables|Default|GetMaxRotate)) 0.0 0.0) false false)))
    (else
      (Timeline|SwingTimeLine Reverse))))

(fn ConstructionScript)