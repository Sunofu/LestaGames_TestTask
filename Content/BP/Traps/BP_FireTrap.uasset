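; Floor trap that damages the player who steps on it, with material swaps signaling each stage.
; Overlap by a "Player"-tagged actor shows the activated material, then after a one-second delay damages the cached player character if still on the trap.
; It flashes a damage material, restores the floor material, and reloads on a timer.
; When reload ends, it fires again if the player remains.
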(event OnComponentBeginOverlap(InteractionCollider)
  (params (OverlappedComponent :type Primitive%20Component%20Object%20Reference) (OtherActor :type Actor%20Object%20Reference) (OtherComp :type Primitive%20Component%20Object%20Reference) (OtherBodyIndex :type Integer) (bFromSweep :type Boolean) (SweepResult :type Hit%20Result%20Structure%20%28by%20ref%29))
  ;[1 1 1] TrapActivate
  (if (Actor|ActorHasTag OtherActor "Player")
    (Variables|Default|SetIsPlayerOnTrap true)
    (CallFunction|DamagePlayer OtherActor)))

(event OnComponentEndOverlap(InteractionCollider)
  (params (OverlappedComponent :type Primitive%20Component%20Object%20Reference) (OtherActor :type Actor%20Object%20Reference) (OtherComp :type Primitive%20Component%20Object%20Reference) (OtherBodyIndex :type Integer))
  ;[1 1 1] TrapDiactivate
  (if (Actor|ActorHasTag OtherActor "Player")
    (Variables|Default|SetIsPlayerOnTrap false)))

(event Custom|damagePlayer
  (params (DamagedActor :type Actor%20Object%20Reference))
  ;[1 1 1] DamagePlayer
  (if (not (Variables|Default|GetIsReloading))
    (Rendering|Material|SetMaterial (Variables|Default|GetStaticMesh) 0 "/Game/Materials/M_ActivatedTrap.M_ActivatedTrap")
    (Utilities|FlowControl|Delay 1.0)
    (if (Variables|Default|GetIsPlayerOnTrap)
      (Default|GetDamage (Variables|Default|GetAs%20BP%20Lesta%20Base%20Character) (Variables|Default|GetDamage)))
    (Rendering|Material|SetMaterial (Variables|Default|GetStaticMesh) 0 "/Game/Materials/M_DamageTrap.M_DamageTrap")
    (bind _returnvalue (Utilities|Time|SetTimerbyEvent (delegate Custom|SetDeafaultMaterialBeforeReload) 0.2))
    (Variables|Default|SetIsReloading true)
    (bind _returnvalue_2 (Utilities|Time|SetTimerbyEvent (delegate Custom|AfterReload) (Variables|Default|GetReloadTime)))))

(event Custom|AfterReload
  ;[1 1 1] DamagePlayer
  (Variables|Default|SetIsReloading false)
  (if (Variables|Default|GetIsPlayerOnTrap)
    (CallFunction|DamagePlayer (stale Custom|damagePlayer DamagedActor))
    (CallFunction|ClearRealoadingTimer)))

(event Custom|SetDeafaultMaterialBeforeReload
  ;[1 1 1] DamagePlayer
  (Rendering|Material|SetMaterial (Variables|Default|GetStaticMesh) 0 "/Game/StarterContent/Materials/M_Basic_Floor.M_Basic_Floor")
  (CallFunction|ClearMaterialTimer))

(event Custom|ClearMaterialTimer
  ;[1 1 1] DamagePlayer
  (Utilities|Time|ClearandInvalidateTimerbyHandle (stale Custom|damagePlayer _returnvalue)))

(event Custom|ClearRealoadingTimer
  ;[1 1 1] DamagePlayer
  (Utilities|Time|ClearandInvalidateTimerbyHandle (stale Custom|damagePlayer _returnvalue_2)))

(event EventBeginPlay
  (bind _asbp_lesta_base_character (Utilities|Casting|CastToBP_Lesta_Base_Character (Game|GetPlayerCharacter 0)))
  (Variables|Default|SetAs%20BP%20Lesta%20Base%20Character _asbp_lesta_base_character))

(fn ConstructionScript)