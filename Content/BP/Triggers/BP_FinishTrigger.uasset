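; BP_FinishTrigger is a level finish trigger that ends the game with a win when the player character reaches it.
; On actor overlap it acts once, guarded by IsActivated, and only for a BP_Lesta_Base_Character.
; It flags the character's IsWin, pauses the game, shows the W_EndGameWidjet end screen and switches the first player controller to UI-only input with a visible cursor.
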(event Collision|EventActorBeginOverlap
  (params (OtherActor :type Actor%20Object%20Reference))
  (bind _returnvalue (Game|GetPlayerController 0))
  (if (not (Variables|Default|GetIsActivated))
    (bind _asbp_lesta_base_character (Utilities|Casting|CastToBP_Lesta_Base_Character OtherActor))
    (Variables|Default|SetIsActivated true)
    (Variables|/Game/BP/Characters/BP_Lesta_Base_Character.BP_Lesta_Base_Character_C|SetIsWin _asbp_lesta_base_character true)
    (Game|SetGamePaused true)
    (bind _returnvalue_2 (UserInterface|CreateWidget "/Game/BP/UI/W_EndGameWidjet.W_EndGameWidjet_C" _returnvalue))
    (UserInterface|Viewport|AddtoViewport _returnvalue_2 0)
    (Variables|/Script/Engine.PlayerController|SetbShowMouseCursor _returnvalue true)
    (Input|SetInputModeUIOnly _returnvalue _returnvalue_2 "DoNotLock" false)))

(fn ConstructionScript)