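; BP_Lesta_playerController is a player controller that handles pausing and the pause menu.
; BeginPlay unpauses the game, sets game-only input and hides the cursor.
; The Pause action toggles an IsPaused flag: pausing creates and shows a new W_PauseMenu with game-and-UI input and a visible cursor.
; Unpausing removes the widget and restores game-only input without a cursor.
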(event EventBeginPlay
  (Game|SetGamePaused false)
  (Input|SetInputModeGameOnly self false)
  (Variables|Default|SetbShowMouseCursor false))

(event Input|ActionEvents|InputActionPause
  (params (Key :type Key%20Structure :default "None"))
  (bind _returnvalue (Game|GetPlayerController 0))
  (:Pressed
    (if (Variables|Default|GetIsPaused)
      (Variables|Default|SetIsPaused false)
      (Widget|RemovefromParent (Variables|Default|GetPauseMenu))
      (Game|SetGamePaused false)
      (Input|SetInputModeGameOnly self false)
      (Variables|Default|SetbShowMouseCursor false)
      (else
        (Variables|Default|SetIsPaused true)
        (bind _returnvalue_2 (UserInterface|CreateWidget "/Game/BP/UI/W_PauseMenu.W_PauseMenu_C" (Game|GetPlayerController 0)))
        (bind _output_get (Variables|Default|SetPauseMenu _returnvalue_2))
        (Game|SetGamePaused true)
        (UserInterface|Viewport|AddtoViewport _output_get 0)
        (Input|SetInputModeGameandUI self 0 "DoNotLock" true false)
        (Input|EnableInput _returnvalue _returnvalue)
        (Variables|Default|SetbShowMouseCursor true)))))

(fn ConstructionScript)